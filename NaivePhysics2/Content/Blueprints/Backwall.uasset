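; Backwall actor that procedurally builds occluder wall geometry in its construction script; its event graph is empty.
; It looks up the wall material from MaterialName and adds a back wall mesh at a fixed X, positioned by YLocation and scaled by ZScale.
; Outside test iterations, it also adds two perpendicular side walls at plus and minus half of XWidth, sharing the mesh, material and height scale.
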(event `self.ReceiveBeginPlay`)

(event `self.ReceiveActorBeginOverlap`
  (params (OtherActor :type "Actor Object Reference")))

(event `self.ReceiveTick`
  (params (DeltaSeconds :type "Float (single-precision)")))

(fn `UserConstructionScript`
  (bind _returnvalue (`NaivePhysicsLib.GetMaterialFromName` (`self.Material Name`)))
  (set `self.Wall Material` _returnvalue)
  (bind _returnvalue_2 (`AddComponent|StaticMeshComponent_15` :`RelativeTransform` (`KismetMathLibrary.MakeTransform` (`KismetMathLibrary.MakeVector` -3140.0 (`self.Y Location`)) (`KismetMathLibrary.MakeRot` 0.0) (`KismetMathLibrary.MakeVector` 15.0 0.75 (`self.Z Scale`))))) ; This is the back wall only
  (`StaticMeshComponent.SetStaticMesh` _returnvalue_2 "/Game/Meshes/OccluderWall.OccluderWall")
  (`PrimitiveComponent.SetMaterial` _returnvalue_2 0 (`self.Wall Material`))
  (if (not (`self.Is Test Iteration`))
    (bind _returnvalue_3 (`AddComponent|StaticMeshComponent_16` :`RelativeTransform` (`KismetMathLibrary.MakeTransform` (`KismetMathLibrary.MakeVector` (* (/ (`self.X Width`) 2.0) -1.0) (- (`self.Y Location`) 200.0)) (`KismetMathLibrary.MakeRot` 0.0 90.0) (`KismetMathLibrary.MakeVector` 6.0 0.75 (`self.Z Scale`)))))
    (`StaticMeshComponent.SetStaticMesh` _returnvalue_3 "/Game/Meshes/OccluderWall.OccluderWall")
    (`PrimitiveComponent.SetMaterial` _returnvalue_3 0 (`self.Wall Material`))
    (bind _returnvalue_4 (`AddComponent|StaticMeshComponent_142` :`RelativeTransform` (`KismetMathLibrary.MakeTransform` (`KismetMathLibrary.MakeVector` (/ (`self.X Width`) 2.0) (- (`self.Y Location`) 200.0)) (`KismetMathLibrary.MakeRot` 0.0 90.0) (`KismetMathLibrary.MakeVector` 6.0 0.75 (`self.Z Scale`)))))
    (`StaticMeshComponent.SetStaticMesh` _returnvalue_4 "/Game/Meshes/OccluderWall.OccluderWall")
    (`PrimitiveComponent.SetMaterial` _returnvalue_4 0 (`self.Wall Material`))))